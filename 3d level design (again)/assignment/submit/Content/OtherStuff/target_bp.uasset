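; Target actor that detects the player by proximity and tracks an alert level over time.
; Overlap begin and end on a Sphere component set DetectionActive when the player character enters or leaves.
; Tick raises AlertMeter by delta time while detection is active and drains it back to zero otherwise, printing debug strings along the way.
; The meter has no upper limit and triggers no further behaviour here.
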(event OnComponentBeginOverlap(Sphere)
  (params (OverlappedComponent :type Primitive%20Component%20Object%20Reference) (OtherActor :type Actor%20Object%20Reference) (OtherComp :type Primitive%20Component%20Object%20Reference) (OtherBodyIndex :type Integer) (bFromSweep :type Boolean) (SweepResult :type Hit%20Result%20Structure%20%28by%20ref%29))
  ;[0.3746 1 0.364] detect player when player too close
  (if (== OtherActor (Game|GetPlayerCharacter 0))
    (bind _output_get (Variables|Default|Setdetection%20active true))
    (Development|PrintString (Utilities|String|ToString(Boolean) _output_get))))

(event OnComponentEndOverlap(Sphere)
  (params (OverlappedComponent :type Primitive%20Component%20Object%20Reference) (OtherActor :type Actor%20Object%20Reference) (OtherComp :type Primitive%20Component%20Object%20Reference) (OtherBodyIndex :type Integer))
  ;[1 0.1698 0.1698] player leave detection zone
  (if (== (Game|GetPlayerCharacter 0) OtherActor)
    (bind _output_get (Variables|Default|Setdetection%20active false))
    (Development|PrintString (Utilities|String|ToString(Boolean) _output_get))))

(event EventTick
  (params (DeltaSeconds :type Float%20%28single-precision%29))
  (CallFunction|PlayerDetected DeltaSeconds)
  (CallFunction|AlertReset DeltaSeconds))

(fn ConstructionScript)

(fn PlayerDetected
  (params (delta%20time :type Float%20%28double-precision%29))
  (if (Variables|Default|Getdetection%20active)
    (bind _output_get (Variables|Default|Setalert%20meter (+ (Variables|Default|Getalert%20meter) delta%20time)))
    (Development|PrintString (Utilities|String|ToString(Float) _output_get))))

(fn AlertReset
  (params (delta%20time :type Float%20%28double-precision%29))
  (if (and (not (Variables|Default|Getdetection%20active)) (> (Variables|Default|Getalert%20meter) 0.0))
    (bind _output_get (Variables|Default|Setalert%20meter (- (Variables|Default|Getalert%20meter) delta%20time)))
    (if (<= _output_get 0.0)
      (Variables|Default|Setalert%20meter 0.0)
      (Development|PrintString "alertness reset"))))